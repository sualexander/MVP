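; Chest interactable Blueprint that opens only once at least three keys have been collected.
; KeyCheck increments the key count, and DoAnimation tests it, printing an opened message or a locked message.
; A locked attempt clears HasInteracted.
; The Animation function only prints a debug string, and the construction script just calls its parent.
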(event `self.DoAnimation`
  (if (>= (`self.NumKeys`) 3)
    (`KismetSystemLibrary.PrintString` "You Opened The Chest!")
    (else
      (`KismetSystemLibrary.PrintString` "Locked")
      (set `self.HasInteracted` false))))

(event `KeyCheck`
  (bind _result (`/Engine/EditorBlueprintResources/StandardMacros.IncrementInt` (`self.NumKeys`))
    (:`  `
      (set `self.NumKeys` _result))))

(fn `Animation`
  (`KismetSystemLibrary.PrintString` "Overided"))

(fn `UserConstructionScript`
  (`parent.UserConstructionScript`))