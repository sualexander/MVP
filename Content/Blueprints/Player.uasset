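; First-person player Blueprint that handles movement, camera look, inventory UI and detection of interactible objects.
; It adds a hotbar on BeginPlay, and the Inventory input toggles the inventory widget and mouse cursor, pausing look and tracing while open.
; UpdateInventory refreshes that widget by removing and recreating it.
; Each Tick traces from the camera, using paired DoOnce gates to notify Interactible actors when the hit state changes.
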(event `self.ReceiveBeginPlay`
  (bind _returnvalue (`|CreateWidget` "/Game/Blueprints/HotBarUI.HotBarUI_C" null (`self.Inventory`) "Empty"))
  (set `self.HotBarUI` _returnvalue)
  (`UserWidget.AddToViewport` _returnvalue 0))

(event `InputAxis|MoveForwardBack`
  (params (AxisValue :type "Float (single-precision)"))
  (`self.AddMovementInput` (`self.GetActorForwardVector`) AxisValue))

(event `InputAction|Inventory`
  (params (Key :type "Key Structure"))
  (bind _returnvalue (`GameplayStatics.GetPlayerController` 0))
  (:`Pressed`
    (bind _output_get (set `self.InventoryIsOpen` (not (`self.InventoryIsOpen`))))
    (if _output_get
      (bind _returnvalue_2 (`|CreateWidget` "/Game/Blueprints/InventoryUI.InventoryUI_C" null (`self.Inventory`) :!label _label))
      (set `self.InventoryUI` _returnvalue_2)
      (`UserWidget.AddToViewport` _returnvalue_2 0)
      (set `PlayerController.bShowMouseCursor` true _returnvalue)
      (else
        (`Widget.RemoveFromParent` _returnvalue_2 :!label _label_2)
        (set `PlayerController.bShowMouseCursor` false _returnvalue)))))

(event `UpdateInventory`
  (`|ExecutionSequence`
    (:`then_0`
      (goto _label_2))
    (:`then_1`
      (goto _label))))

(event `InputAxis|MoveLeftRight`
  (params (AxisValue :type "Float (single-precision)"))
  (`self.AddMovementInput` (`self.GetActorRightVector`) AxisValue))

(event `ResetDoOnce2`
  (goto _label_4 :!via `Reset`))

(event `ResetDoOnce`
  (goto _label_3 :!via `Reset`))

(event `self.ReceiveTick`
  (params (DeltaSeconds :type "Float (single-precision)"))
  (bind _camera (`self.Camera`))
  (bind _returnvalue (`SceneComponent.K2_GetComponentLocation` _camera))
  (if (not (`self.InventoryIsOpen`))
    (`self.AddControllerYawInput` (`self.GetInputAxisKeyValue`))
    (`self.AddControllerPitchInput` (* (`self.GetInputAxisKeyValue`) -1.0))
    (bind _outhit (`KismetSystemLibrary.LineTraceSingleForObjects` _returnvalue (+ _returnvalue (* (`KismetMathLibrary.GetForwardVector` (`SceneComponent.K2_GetComponentRotation` _camera)) 500)) (`|MakeArray` "ObjectTypeQuery7" :!type "EObjectTypeQuery Enum")))
    (bind (_bblockinghit _binitialoverlap _time _distance _location _impactpoint _normal _impactnormal _physmat _hitactor) (`GameplayStatics.BreakHitResult` _outhit))
    (if (!= (`self.switchBoolean`) _bblockinghit)
      (`self.ResetDoOnce`))
    (if _bblockinghit
      (`self.ResetDoOnce2`)
      (`/Engine/EditorBlueprintResources/StandardMacros.DoOnce` false :!label _label_3
        (:`Completed`
          (set `self.switchBoolean` _bblockinghit)
          (bind _output_get (set `self.Name` _hitactor))))
      (else
        (`/Engine/EditorBlueprintResources/StandardMacros.DoOnce` false :!label _label_4
          (:`Completed`
            _))))
    (bind _asinteractible (cast `/Game/Blueprints/Interactible` _output_get))
    (if (`KismetSystemLibrary.IsValid` _asinteractible)
      (`/Game/Blueprints/Interactible.UpdateRayCastInteractible` _asinteractible _bblockinghit (`KismetStringLibrary.Conv_ObjectToString` _output_get)))))

(fn `UserConstructionScript`)