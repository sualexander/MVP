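; Base interactible object that shows an InteractibleUI prompt on player raycast and can require a Key item from the hotbar.
; Use places or retrieves the item through the player's inventory, refreshing the hotbar and calling the empty UseUpdate hook.
; Interact checks any required item, then locks further prompting and runs DoAnimation, which moves the root and plays player narration.
; UpdatePrompt rebuilds the widget through a gate and short delay.
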(event `UpdateRayCastInteractible`
  (params (True :type Boolean) (Name :type String))
  (bind _returnvalue (`GameplayStatics.GetPlayerController` 0))
  (bind _itemused_name (break `/Game/Item` (`self.ItemUsed`)))
  (bind _hasused (`self.HasUsed`))
  (bind _returnvalue_2 (`KismetTextLibrary.Conv_TextToString` _itemused_name))
  (if (not (`self.HasInteracted`))
    (bind _asplayer (cast `/Game/Blueprints/BaseObjects/Player` (`GameplayStatics.GetPlayerPawn` 0)))
    (if True :!label _label
      (`/Engine/EditorBlueprintResources/StandardMacros.Gate` false :!label _label_2
        (:`Exit`
          (`self.EnableInput` _returnvalue)
          (bind _returnvalue_3 (`|CreateWidget` "/Game/Blueprints/BaseObjects/InteractibleUI.InteractibleUI_C"))
          (bind (_hotbaritem_name _hotbaritem_thumbnail _hotbaritem_pickupable _hotbaritem_class) (break `/Game/Item` (`/Game/Blueprints/BaseObjects/Inventory.HotBarItem` (`/Game/Blueprints/BaseObjects/Player.Inventory` _asplayer))))
          (bind _returnvalue_4 (not (`KismetTextLibrary.TextIsEmpty` _hotbaritem_name)))
          (bind _returnvalue_5 (`KismetStringLibrary.EqualEqual_StrStr` _hotbaritem_class "Key"))
          (set `/Game/Blueprints/BaseObjects/InteractibleUI.Interactible Name` (select `bool` (`self.CanInteract`) :`false` (select `bool` (or (and _returnvalue_4 _returnvalue_5) _hasused) :`true` (`KismetTextLibrary.Conv_StringToText` (`KismetStringLibrary.Concat_StrStr` (`KismetMathLibrary.SelectString` "Press \"V\" To Remove" (`KismetStringLibrary.Concat_StrStr` "Press \"V\" To Use With" " " Name) _hasused) " " _returnvalue_2))) :`true` (select `bool` (or (and _returnvalue_4 (`self.RequiresItem`) _returnvalue_5) (`self.HasUsed`)) :`false` (`KismetTextLibrary.Conv_StringToText` (`KismetStringLibrary.Concat_StrStr` "Press \"F\" to Interact With" " " Name)) :`true` (`KismetTextLibrary.Conv_StringToText` (`KismetStringLibrary.Concat_StrStr` "Press \"F\" to Interact WIth" " " Name " " (select `bool` _hasused :`false` "Or Press \"V\" to Use" :`true` "Or Press \"V\" to Remove") " " _returnvalue_2)))) _returnvalue_3)
          (`UserWidget.AddToViewport` _returnvalue_3 0)))
      (else
        (`self.DisableInput` _returnvalue :!label _label_3)
        (bind _foundwidgets (`WidgetBlueprintLibrary.GetAllWidgetsOfClass` "/Game/Blueprints/BaseObjects/InteractibleUI.InteractibleUI_C"))
        (for _array_element _foundwidgets
          (`Widget.RemoveFromParent` _array_element))))))

(event `UpdatePrompt`
  (`|ExecutionSequence`
    (:`then_0`
      (goto _label_2 :!via `Close`))
    (:`then_1`
      (goto _label_3))
    (:`then_2`
      (`KismetSystemLibrary.Delay` 0.2)
      (`|ExecutionSequence`
        (:`then_0`
          (goto _label_2 :!via `Open`))
        (:`then_1`
          (goto _label))))))

(event `RemovePrompt`
  (goto _label_3))

(event `UpdateInteract`
  (if (== (`self.RequiredItem`) (`.Pickupable_13_DBC8569B4C0E00B7E679FFAF73D70833` (break `/Game/Item` (stale `InputAction|Use` _output_get))))
    (set `self.HasInteracted` true :!label _label_4)
    (`self.DoAnimation`)))

(event `InputAction|Interact`
  (params (Key :type "Key Structure"))
  (bind _itemused_name (break `/Game/Item` (`self.ItemUsed`)))
  (:`Pressed`
    (if (`self.CanInteract`)
      (`self.UpdatePrompt`)
      (if (`self.RequiresItem`)
        (if (`KismetTextLibrary.TextIsEmpty` _itemused_name)
          (`KismetSystemLibrary.PrintString` "Requires Item")
          (elif (== (`self.RequiredItem`) (`.Pickupable_13_DBC8569B4C0E00B7E679FFAF73D70833` (break `/Game/Item` (stale `InputAction|Use` _output_get))))
            (goto _label_4)
            (else
              (`KismetSystemLibrary.PrintString` "Wrong Item"))))
        (else
          (goto _label_4))))))

(event `InputAction|Use`
  (params (Key :type "Key Structure"))
  (bind _hasused (`self.HasUsed`))
  (:`Pressed`
    (bind _inventory (`/Game/Blueprints/BaseObjects/Player.Inventory` (stale `UpdateRayCastInteractible` _asplayer)))
    (bind (_hotbaritem_name _hotbaritem_thumbnail _hotbaritem_pickupable _hotbaritem_class) (break `/Game/Item` (`/Game/Blueprints/BaseObjects/Inventory.HotBarItem` _inventory)))
    (if (`KismetStringLibrary.EqualEqual_StrStr` _hotbaritem_class "Key")
      (`self.UpdatePrompt`)
      (bind _returnvalue (`KismetTextLibrary.TextIsEmpty` _hotbaritem_name))
      (if _returnvalue
        (if _hasused :!label _label_5
          (if _hasused :!label _label_6
            (if _returnvalue
              (`KismetSystemLibrary.PrintString` "Item Retrieved")
              (set `/Game/Blueprints/BaseObjects/Inventory.HotBarItem` (`self.ItemUsed`) _inventory)
              (bind _hotbarui (`/Game/Blueprints/BaseObjects/Player.HotBarUI` (stale `UpdateRayCastInteractible` _asplayer)))
              (`/Game/Blueprints/BaseObjects/HotBarUI.Replace` _hotbarui)
              (set `self.ItemUsed` (make `/Game/Item` ""))
              (set `self.HasUsed` false)
              (else
                (`KismetSystemLibrary.PrintString` "Hotbar Is Full")))
            (elif (`self.RequiresItem`)
              (bind _output_get (set `self.ItemUsed` (`/Game/Blueprints/BaseObjects/Inventory.HotBarItem` _inventory)))
              (set `/Game/Blueprints/BaseObjects/Inventory.HotBarItem` (make `/Game/Item` "") _inventory)
              (`/Game/Blueprints/BaseObjects/HotBarUI.Replace` _hotbarui)
              (set `self.HasUsed` true)
              (`self.UseUpdate`)
              (else
                (`KismetSystemLibrary.PrintString` "Cannot Use Item With Object"))))
          (else
            (`KismetSystemLibrary.PrintString` "No Item To Use")))
        (else
          (goto _label_6)))
      (elif _returnvalue
        (goto _label_5)))))

(event `UseUpdate`)

(event `DoAnimation`
  (bind _defaultsceneroot (`self.DefaultSceneRoot`))
  (bind _transform_location (`KismetMathLibrary.BreakTransform` (`self.Transform`)))
  (`self.RemovePrompt`)
  (`KismetSystemLibrary.MoveComponentTo` _defaultsceneroot (+ (`SceneComponent.K2_GetComponentLocation` _defaultsceneroot) _transform_location) (struct) false false 0.5)
  (bind _asplayer (cast `/Game/Blueprints/BaseObjects/Player` (`GameplayStatics.GetPlayerPawn` 0)))
  (`/Game/Audio/NarrationPlayer.PlaySound` (`/Game/Blueprints/BaseObjects/Player.NarrationPlayer` _asplayer)))

(fn `UserConstructionScript`)