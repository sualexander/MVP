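; Inventory Blueprint that stores picked-up items and manages a single hotbar item the player can use.
; Adding items to inventory or hotbar adjusts an item counter, and hotbar assignment also refreshes the player's HotBarUI.
; UseItem branches on item class, toggling the player's spotlight for Flashlight or opening and closing an image widget for Note.
; Hotbar changes call UpdateUsedItem, which hides the light, removes the note and flips the note toggle.
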(event `AddToInventory`
  (params (Item :type "/Game/Item Structure"))
  (set `self.MaxItems` (+ (`self.MaxItems`) 1))
  (`KismetArrayLibrary.Array_Add` (`self.InventoryItems`) Item))

(event `AddToHotBar`
  (params (Item :type "/Game/Item Structure"))
  (set `self.MaxItems` (- (`self.MaxItems`) 1))
  (set `self.HotBarItem` Item)
  (bind _asplayer (cast `/Game/Blueprints/BaseObjects/Player` (`GameplayStatics.GetPlayerPawn` 0)))
  (`/Game/Blueprints/BaseObjects/HotBarUI.Replace` (`/Game/Blueprints/BaseObjects/Player.HotBarUI` _asplayer))
  (`self.UpdateUsedItem`))

(event `UpdateUsedItem`
  (`SceneComponent.SetVisibility` (`Actor.GetComponentByClass` (stale `UseItem` _asplayer) "/Script/Engine.SpotLightComponent") false false)
  (`Widget.RemoveFromParent` (stale `UseItem` _returnvalue) :!label _label)
  (set `self.Condition` (not (`self.Condition`)) :!label _label_2))

(event `UseItem`
  (bind (_hotbaritem_name _hotbaritem_thumbnail _hotbaritem_pickupable _hotbaritem_class _hotbaritem_noteimage) (break `/Game/Item` (`self.HotBarItem`)))
  (switch `string` _hotbaritem_class
    (:`Flashlight`
      (bind _asplayer (cast `/Game/Blueprints/BaseObjects/Player` (`GameplayStatics.GetPlayerPawn` 0)))
      (`SceneComponent.ToggleVisibility` (`Actor.GetComponentByClass` _asplayer "/Script/Engine.SpotLightComponent") false))
    (:`Note`
      (if (`self.Condition`)
        (bind _returnvalue (`|CreateWidget` "/Game/Blueprints/BaseObjects/NoteUI.NoteUI_C" null _hotbaritem_noteimage))
        (`UserWidget.AddToViewport` _returnvalue 0)
        (goto _label_2)
        (else
          (goto _label))))))